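; Modular mech Blueprint that assembles its appearance from six skeletal mesh body parts when play begins.
; BeginPlay calls CheckAndGetParts, then applies each valid result to its component, leaving a component unchanged when its part is invalid.
; The head goes on the main Mesh component, while the torso, arms and legs each have their own component.
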(event EventBeginPlay
  (bind _returnvalue (Class|PMCharacter|CheckandGetParts))
  (Utilities|IsValid (.Head (Utilities|Struct|BreakMeshInfo _returnvalue))
    (:Is%20Valid
      (Components|SkeletalMesh|SetSkeletalMeshAsset (Variables|Character|GetMesh) (.Head (Utilities|Struct|BreakMeshInfo _returnvalue))))
    (:Is%20Not%20Valid
      _))
  (Utilities|IsValid (.Torso (Utilities|Struct|BreakMeshInfo _returnvalue))
    (:Is%20Valid
      (Components|SkeletalMesh|SetSkeletalMeshAsset (Variables|Default|GetTorso) (.Torso (Utilities|Struct|BreakMeshInfo _returnvalue))))
    (:Is%20Not%20Valid
      _))
  (Utilities|IsValid (.ArmLeft (Utilities|Struct|BreakMeshInfo _returnvalue))
    (:Is%20Valid
      (Components|SkeletalMesh|SetSkeletalMeshAsset (Variables|Default|GetArmLeft) (.ArmLeft (Utilities|Struct|BreakMeshInfo _returnvalue))))
    (:Is%20Not%20Valid
      _))
  (Utilities|IsValid (.ArmRight (Utilities|Struct|BreakMeshInfo _returnvalue))
    (:Is%20Valid
      (Components|SkeletalMesh|SetSkeletalMeshAsset (Variables|Default|GetArmRight) (.ArmRight (Utilities|Struct|BreakMeshInfo _returnvalue))))
    (:Is%20Not%20Valid
      _))
  (Utilities|IsValid (.LegLeft (Utilities|Struct|BreakMeshInfo _returnvalue))
    (:Is%20Valid
      (Components|SkeletalMesh|SetSkeletalMeshAsset (Variables|Default|GetLegLeft) (.LegLeft (Utilities|Struct|BreakMeshInfo _returnvalue))))
    (:Is%20Not%20Valid
      _))
  (Utilities|IsValid (.LegRight (Utilities|Struct|BreakMeshInfo _returnvalue))
    (:Is%20Valid
      (Components|SkeletalMesh|SetSkeletalMeshAsset (Variables|Default|GetLegRight) (.LegRight (Utilities|Struct|BreakMeshInfo _returnvalue))))))

(event Collision|EventActorBeginOverlap
  (params (OtherActor :type Actor%20Object%20Reference)))

(event EventTick
  (params (DeltaSeconds :type Float%20%28single-precision%29)))

(fn ConstructionScript)